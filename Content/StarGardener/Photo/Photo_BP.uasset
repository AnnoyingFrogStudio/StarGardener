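; Photo-mode pawn that the player possesses to look around, take pictures and browse a photo gallery, then exits by handing possession back and destroying itself.
; Taking a picture captures the scene into a fresh render target, shows it in a PhotoDisplay widget and fires the TakenPhoto dispatcher.
; That dispatcher, bound on possession, appends photos to the referenced gallery array, which IA_Drop toggles on screen as a PhotoGallery widget.
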(event Custom|AddToGallery
  (params (Photo :type Texture%20Render%20Target%202D%20Object%20Reference))
  (Utilities|Array|Add (Variables|/Game/StarGardener/Photo/PDA_PhotoGalleryRef.PDA_PhotoGalleryRef_C|GetPhotoGallery (Variables|Default|GetPhotoGalleryReference)) Photo))

(event Input|EnhancedActionEvents|EnhancedInputActionIA_TakePicture
  (params (ActionValue :type Boolean) (ElapsedSeconds :type Float%20%28double-precision%29) (TriggeredSeconds :type Float%20%28double-precision%29) (InputAction :type Input%20Action%20Object%20Reference :default "/Game/StarGardener/CharacterController/Input/Actions/IA_TakePicture.IA_TakePicture"))
  (bind _scenecapturecomponent2d (Variables|Default|GetSceneCaptureComponent2D))
  (:Started
    (bind _returnvalue (Rendering|CreateRenderTarget2D 1920 1080 "RTF_RGBA16f"))
    (bind _output_get (Variables|/Script/Engine.SceneCaptureComponent2D|SetTextureTarget _scenecapturecomponent2d _returnvalue))
    (bind _returnvalue_2 (UserInterface|CreateWidget "/Game/StarGardener/Photo/PhotoDisplay.PhotoDisplay_C" 0 _output_get))
    (Rendering|SceneCapture|CaptureScene _scenecapturecomponent2d :!class /Script/Engine.SceneCaptureComponent2D)
    (UserInterface|Viewport|AddtoViewport _returnvalue_2 0)
    (Default|CallTakenPhoto (Variables|/Script/Engine.SceneCaptureComponent2D|GetTextureTarget (Variables|Default|GetSceneCaptureComponent2D)))))

(event Input|EnhancedActionEvents|EnhancedInputActionIA_Look
  (params (ActionValue :type Vector%202D%20Structure) (ElapsedSeconds :type Float%20%28double-precision%29) (TriggeredSeconds :type Float%20%28double-precision%29) (InputAction :type Input%20Action%20Object%20Reference :default "/Game/StarGardener/CharacterController/Input/Actions/IA_Look.IA_Look"))
  ;[1 1 1] Camera controls
  (:Triggered
    (Pawn|Input|AddControllerYawInput (.x ActionValue))
    (Pawn|Input|AddControllerPitchInput (.y ActionValue))))

(event Input|EnhancedActionEvents|EnhancedInputActionIA_Drop
  (params (ActionValue :type Boolean) (ElapsedSeconds :type Float%20%28double-precision%29) (TriggeredSeconds :type Float%20%28double-precision%29) (InputAction :type Input%20Action%20Object%20Reference :default "/Game/StarGardener/CharacterController/Input/Actions/IA_Drop.IA_Drop"))
  (:Started
    (bind _gallery (Variables|Default|GetGallery)
      (:then
        (Widget|RemovefromParent _gallery)
        (Variables|Default|SetGallery 0))
      (:else
        (bind _returnvalue (UserInterface|CreateWidget "/Game/StarGardener/Photo/PhotoGallery.PhotoGallery_C" 0 (Variables|/Game/StarGardener/Photo/PDA_PhotoGalleryRef.PDA_PhotoGalleryRef_C|GetPhotoGallery (Variables|Default|GetPhotoGalleryReference))))
        (bind _output_get (Variables|Default|SetGallery _returnvalue))
        (UserInterface|Viewport|AddtoViewport _output_get 0)))))

(event Input|EnhancedActionEvents|EnhancedInputActionIA_ChangeMode
  (params (ActionValue :type Boolean) (ElapsedSeconds :type Float%20%28double-precision%29) (TriggeredSeconds :type Float%20%28double-precision%29) (InputAction :type Input%20Action%20Object%20Reference :default "/Game/StarGardener/CharacterController/Input/Actions/IA_ChangeMode.IA_ChangeMode"))
  ;[1 1 1] Return to base character
  (:Started
    (Default|ChangerPossess (Variables|Default|GetModeChanger) (Variables|Default|GetPlayer))
    (Actor|DestroyActor)))

(event EventBeginPlay
  ;[1 1 1] Begin play
  (bind _asplayer_controller (Utilities|Casting|CastToPlayerController (Pawn|GetController)))
  (Utilities|IsValid (PlayerController|LocalPlayerSubsystems|GetEnhancedInputLocalPlayerSubsystem _asplayer_controller)
    (:Is%20Valid
      (Input|AddMappingContext (PlayerController|LocalPlayerSubsystems|GetEnhancedInputLocalPlayerSubsystem _asplayer_controller) "/Game/StarGardener/CharacterController/Input/IMC_Default.IMC_Default" 0 "(bIgnoreAllPressedKeysUntilRelease=True,bForceImmediately=False)"))))

(event EventPossessed
  (params (NewController :type Controller%20Object%20Reference))
  (EventDispatchers|BindEventtoTakenPhoto (delegate Custom|AddToGallery)))

(fn ConstructionScript)