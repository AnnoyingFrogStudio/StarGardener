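; Scene capture actor in StarGardener's virtual textures, apparently for recording player position over trail areas.
; BeginPlay restricts the capture to ITrailArea actors and sets ortho width and view distance from camera size and far cut.
; Tick passes the parameter collection's player Position to IsTargetInBox, whose box test is unconnected, and captures manually when it returns true.
; ClearRTData clears PositionRT, while debug box drawing is disconnected.
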(event Custom|DRAW%20DEBUGS
  (params (Color%20Pick :type Boolean)))

(event Custom|CapturePosition
  (Rendering|SceneCapture|CaptureScene (Variables|Default|GetSceneCaptureComponent2D) :!class /Script/Engine.SceneCaptureComponent2D))

(event Custom|Update%20Size
  (bind _scenecapturecomponent2d (Variables|Default|GetSceneCaptureComponent2D))
  (Variables|/Script/Engine.SceneCaptureComponent2D|SetOrthoWidth _scenecapturecomponent2d (Math|Conversions|ToFloat(Integer) (Variables|Default|GetCameraSize)))
  (Variables|/Script/Engine.SceneCaptureComponent|SetMaxViewDistanceOverride _scenecapturecomponent2d (Math|Conversions|ToFloat(Integer) (Variables|Default|GetCameraFarCut))))

(event Custom|Clear%20RT%20Data
  (bind _position_rt (Variables|Default|GetPosition_RT))
  (Rendering|ClearRenderTarget2D _position_rt (Variables|/Script/Engine.TextureRenderTarget2D|GetClearColor _position_rt)))

(event EventBeginPlay
  (bind _outactors (Actor|GetAllActorswithInterface "/Game/StarGardener/VirtualTextures/ITrailArea.ITrailArea_C"))
  (CallFunction|InitSceneCapture _outactors))

(event EventTick
  (params (DeltaSeconds :type Float%20%28single-precision%29))
  (bind _returnvalue (Rendering|Material|GetVectorParameterValue "/Game/StarGardener/VirtualTextures/Player_MatParamCollection.Player_MatParamCollection" "Position" :!class /Script/Engine.KismetMaterialLibrary))
  (CallFunction|DRAWDEBUGS (Utilities|IsTargetinBox (Math|Conversions|ToVector(LinearColor) _returnvalue) (Transformation|GetActorLocation)))
  (if (Utilities|IsTargetinBox (Math|Conversions|ToVector(LinearColor) _returnvalue) (Transformation|GetActorLocation))
    (CallFunction|CapturePosition)))

(fn ConstructionScript)

(fn InitSceneCapture
  (params (Show%20Only%20Actor :type Array%20of%20Actor%20Object%20References))
  (Variables|/Script/Engine.SceneCaptureComponent|SetShowOnlyActors (Variables|Default|GetSceneCaptureComponent2D) Show%20Only%20Actor)
  (CallFunction|UpdateSize))