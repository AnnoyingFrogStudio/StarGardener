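; Photo-mode pawn with look controls, which hands possession back to the player character and destroys itself on mode change.
; Taking a picture captures the scene to a screen-sized render target, exports it as a timestamped PNG, displays it and adds it to the gallery reference.
; A toggled widget shows that gallery, while saved PNGs load into a separate texture array on BeginPlay.
; Registered POI components are printed as on-screen at each shot.
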(event Custom|AddToGallery
  (params (Photo :type Texture%20Render%20Target%202D%20Object%20Reference))
  ;[1 1 1] Add photo to gallery
  (Utilities|Array|Add (Variables|/Game/StarGardener/Object/Photo/PDA_PhotoGalleryRef.PDA_PhotoGalleryRef_C|GetPhotoGallery (Variables|Default|GetPhotoGalleryReference)) Photo))

(event Custom|Close%20Gallery
  ;[1 1 1] Show / Hide Photo Gallery
  (bind _gallery (Variables|Default|GetGallery)
    (:then
      (Widget|RemovefromParent (stale Input|EnhancedActionEvents|EnhancedInputActionIA_Drop _gallery))
      (Variables|Default|SetGallery 0))
    (:else)))

(event Custom|GetExistingPhotos
  ;[1 1 1] Get Photos from file
  (bind _foundfiles (Class|BlueprintFileUtilsBPLibrary|FindFiles (Utilities|GetPhotosPath) ".png"))
  (for _array_element _foundfiles
    (bind _returnvalue (Class|KismetRenderingLibrary|ImportFileasTexture2D _array_element))
    (Utilities|Array|Add (Variables|Default|GetCurentPhotoTexture) _returnvalue)))

(event Custom|AddPOI
  (params (Component :type POI%20Component%20Object%20Reference))
  ;[1 1 1] Add / Remove POI component
  (Utilities|Array|AddUnique (Variables|Default|GetPOIList) Component))

(event Custom|RemovePOI
  (params (Component :type POI%20Component%20Object%20Reference))
  ;[1 1 1] Add / Remove POI component
  (Utilities|Array|RemoveItem (Variables|Default|GetPOIList) Component))

(event Custom|ShowPOIOnScreen
  ;[1 1 1] Print something if a poi is on the picture
  (for _array_element (Variables|Default|GetPOIList)
    (Development|PrintString (Utilities|String|Append (Utilities|GetDisplayName (Components|GetOwner _array_element)) " is on Screen!"))))

(event Input|EnhancedActionEvents|EnhancedInputActionIA_TakePicture
  (params (ActionValue :type Boolean) (ElapsedSeconds :type Float%20%28double-precision%29) (TriggeredSeconds :type Float%20%28double-precision%29) (InputAction :type Input%20Action%20Object%20Reference :default "/Game/StarGardener/Object/CharacterController/Input/Actions/IA_TakePicture.IA_TakePicture"))
  (bind _returnvalue (Math|DateTime|Now))
  (bind _scenecapturecomponent2d (Variables|Default|GetSceneCaptureComponent2D))
  (bind (_year _month _day _hour _minute _second _millisecond) (Math|DateTime|BreakDateTime _returnvalue))
  ;[1 1 1] TakePhoto
  (:Started
    (bind _returnvalue_2 (Settings|GetGameUserSettings))
    (bind _returnvalue_3 (Rendering|CreateRenderTarget2D (.x (Class|GameUserSettings|GetScreenResolution _returnvalue_2)) (.y (Class|GameUserSettings|GetScreenResolution _returnvalue_2)) "RTF_RGBA8_SRGB"))
    (Variables|/Script/Engine.TextureRenderTarget|SetTargetGamma _returnvalue_3 2.0)
    (bind _output_get (Variables|/Script/Engine.SceneCaptureComponent2D|SetTextureTarget _scenecapturecomponent2d _returnvalue_3))
    (bind _returnvalue_4 (UserInterface|CreateWidget "/Game/StarGardener/Object/Photo/PhotoDisplay.PhotoDisplay_C" 0 _output_get))
    (Rendering|SceneCapture|CaptureScene _scenecapturecomponent2d :!class /Script/Engine.SceneCaptureComponent2D)
    (Rendering|ExportRenderTarget (Variables|/Script/Engine.SceneCaptureComponent2D|GetTextureTarget (Variables|Default|GetSceneCaptureComponent2D)) (Utilities|GetPhotosPath) (Utilities|String|Append (Utilities|String|Append (Utilities|String|ToString(Integer) _second) "_" (Utilities|String|ToString(Integer) _minute) "_" (Utilities|String|ToString(Integer) _hour) "_" (Utilities|String|ToString(Integer) _day) "_" (Utilities|String|ToString(Integer) _month) "_" (Utilities|String|ToString(Integer) _year) "_" (Utilities|String|ToString(Integer) _millisecond)) ".png"))
    (UserInterface|Viewport|AddtoViewport _returnvalue_4 0)
    (CallFunction|AddtoGallery (Variables|/Script/Engine.SceneCaptureComponent2D|GetTextureTarget (Variables|Default|GetSceneCaptureComponent2D)))
    (CallFunction|ShowPOIonScreen)))

(event Input|EnhancedActionEvents|EnhancedInputActionIA_Look
  (params (ActionValue :type Vector%202D%20Structure) (ElapsedSeconds :type Float%20%28double-precision%29) (TriggeredSeconds :type Float%20%28double-precision%29) (InputAction :type Input%20Action%20Object%20Reference :default "/Game/StarGardener/Object/CharacterController/Input/Actions/IA_Look.IA_Look"))
  ;[1 1 1] Camera controls
  (:Triggered
    (Pawn|Input|AddControllerYawInput (.x ActionValue))
    (Pawn|Input|AddControllerPitchInput (.y ActionValue))))

(event Input|EnhancedActionEvents|EnhancedInputActionIA_Drop
  (params (ActionValue :type Boolean) (ElapsedSeconds :type Float%20%28double-precision%29) (TriggeredSeconds :type Float%20%28double-precision%29) (InputAction :type Input%20Action%20Object%20Reference :default "/Game/StarGardener/Object/CharacterController/Input/Actions/IA_Drop.IA_Drop"))
  ;[1 1 1] Show / Hide Photo Gallery
  (:Started
    (bind _gallery (Variables|Default|GetGallery)
      (:then
        (Widget|RemovefromParent _gallery)
        (Variables|Default|SetGallery 0))
      (:else
        (bind _returnvalue (UserInterface|CreateWidget "/Game/StarGardener/Object/Photo/PhotoGallery.PhotoGallery_C" 0 (Variables|/Game/StarGardener/Object/Photo/PDA_PhotoGalleryRef.PDA_PhotoGalleryRef_C|GetPhotoGallery (Variables|Default|GetPhotoGalleryReference))))
        (bind _output_get (Variables|Default|SetGallery _returnvalue))
        (UserInterface|Viewport|AddtoViewport _output_get 0)))))

(event Input|EnhancedActionEvents|EnhancedInputActionIA_ChangeMode
  (params (ActionValue :type Boolean) (ElapsedSeconds :type Float%20%28double-precision%29) (TriggeredSeconds :type Float%20%28double-precision%29) (InputAction :type Input%20Action%20Object%20Reference :default "/Game/StarGardener/Object/CharacterController/Input/Actions/IA_ChangeMode.IA_ChangeMode"))
  (bind _player (Variables|Default|GetPlayer))
  ;[1 1 1] Return to base character
  (:Started
    (bind _asice_skatin_bp (Utilities|Casting|CastToIceSkatin_BP _player)
      (:then
        (Rendering|SetVisibility (Variables|/Script/Engine.Character|GetMesh _asice_skatin_bp) true false)
        (Rendering|SetVisibility (Variables|/Game/StarGardener/Object/BackPack/BackPack.BackPack_C|GetBackpack (Variables|/Game/StarGardener/Object/CharacterController/IceSkatin_BP.IceSkatin_BP_C|GetBackPack _asice_skatin_bp)) true false)
        (Rendering|SetVisibility (Variables|/Game/StarGardener/Object/BackPack/BackPack.BackPack_C|GetPollen (Variables|/Game/StarGardener/Object/CharacterController/IceSkatin_BP.IceSkatin_BP_C|GetBackPack _asice_skatin_bp)) true false))
      (:CastFailed
        _))
    (Default|ChangerPossess (Variables|Default|GetModeChanger) _player)
    (CallFunction|CloseGallery)
    (Actor|DestroyActor)))

(event EventBeginPlay
  ;[1 1 1] Begin play
  (CallFunction|GetExistingPhotos)
  (bind _asplayer_controller (Utilities|Casting|CastToPlayerController (Pawn|GetController)))
  (Utilities|IsValid (PlayerController|LocalPlayerSubsystems|GetEnhancedInputLocalPlayerSubsystem _asplayer_controller)
    (:Is%20Valid
      (Input|AddMappingContext (PlayerController|LocalPlayerSubsystems|GetEnhancedInputLocalPlayerSubsystem _asplayer_controller) "/Game/StarGardener/Object/CharacterController/Input/IMC_Default.IMC_Default" 0 "(bIgnoreAllPressedKeysUntilRelease=True,bForceImmediately=False)"))))

(fn ConstructionScript)