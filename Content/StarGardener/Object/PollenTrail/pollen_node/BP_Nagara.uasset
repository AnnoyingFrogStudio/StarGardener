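; Pollen node that sends a Niagara pollen effect flying to the player when the ice-skating character overlaps its sphere.
; The overlap replaces any live effect with a new one and starts a timeline.
; The timeline lerps the effect from the sphere to the live position of the player mesh's niagaraSocket, then destroys it.
; ActivateParticle and DeactivateParticle are empty, and the vector parameter write has no variable name set.
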(event OnComponentBeginOverlap(Sphere)
  (params (OverlappedComponent :type Primitive%20Component%20Object%20Reference) (OtherActor :type Actor%20Object%20Reference) (OtherComp :type Primitive%20Component%20Object%20Reference) (OtherBodyIndex :type Integer) (bFromSweep :type Boolean) (SweepResult :type Hit%20Result%20Structure%20%28by%20ref%29))
  (Utilities|Casting|CastToBP_CharacterIceSkating OtherActor)
  (CallFunction|SpawnPollenFX))

(event Custom|SpawnPollenFX
  (if (Utilities|IsValid (Variables|Default|GetNiagaraSystem))
    (Components|DestroyComponent (Variables|Default|GetNiagaraSystem)))
  (Variables|Default|Setfirst%20location (Transformation|GetWorldLocation (Variables|Default|GetSphere)))
  (bind _returnvalue (Niagara|SpawnSystemAttached "/Game/StarGardener/Object/PollenTrail/pollen_node/pollen_test.pollen_test" (Variables|Default|GetDefaultSceneRoot) "None" "0, 0, 0" "0, 0, 0" "KeepRelativeOffset" false))
  (Variables|Default|SetNiagaraSystem _returnvalue)
  (bind _newtrack_0 (Timeline|Timeline PlayFromStart)
    (:Update
      (Niagara|SetNiagaraVariable(Vector3) (Variables|Default|GetNiagaraSystem) "None" (Math|Vector|Lerp(Vector) (Variables|Default|Getfirst%20location) (Transformation|GetSocketLocation (Actor|GetComponentbyClass (Game|GetPlayerCharacter 0) "/Script/Engine.SkeletalMeshComponent") "niagaraSocket") _newtrack_0))
      (Transformation|SetWorldLocation (Variables|Default|GetNiagaraSystem) (Math|Vector|Lerp(Vector) (Variables|Default|Getfirst%20location) (Transformation|GetSocketLocation (Actor|GetComponentbyClass (Game|GetPlayerCharacter 0) "/Script/Engine.SkeletalMeshComponent") "niagaraSocket") _newtrack_0) false false))
    (:Finished
      (Components|DestroyComponent (Variables|Default|GetNiagaraSystem)))))

(event Custom|ActivateParticle)

(event Custom|DeactivateParticle)

(fn ConstructionScript)