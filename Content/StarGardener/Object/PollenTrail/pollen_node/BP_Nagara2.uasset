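; Pollen node actor for the pollen trail that hosts a Niagara pollen effect.
; On BeginPlay it spawns the effect attached to its root at the Sphere's world location, attempts activation and disables actor collision.
; ActivateParticle switches the stored Niagara component on or off according to the IsActive flag, while DeactivateParticle reuses the off branch.
; Both print debug strings, and a component-destroy step is left unconnected.
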(event Custom|SpawnPollenFX
  (if (Utilities|IsValid (Variables|Default|GetNiagaraSystem))
    _
    (else
      _))
  (bind _output_get (Variables|Default|Setfirst%20location (Transformation|GetWorldLocation (Variables|Default|GetSphere))))
  (bind _returnvalue (Niagara|SpawnSystemAttached "/Game/StarGardener/Object/PollenTrail/pollen_node/pollen_test.pollen_test" (Variables|Default|GetDefaultSceneRoot) "None" _output_get "0, 0, 0" "KeepWorldPosition" false))
  (Variables|Default|SetNiagaraSystem _returnvalue))

(event Custom|ActivateParticle
  (bind _niagarasystem (Variables|Default|GetNiagaraSystem))
  (Utilities|IsValid _niagarasystem
    (:Is%20Valid
      (if (Variables|Default|GetisActive)
        (Components|Activation|Activate _niagarasystem false)
        (Development|PrintString "Activate")
        (else
          (Components|Activation|Deactivate _niagarasystem)
          (Development|PrintString "Deactivate"))))))

(event Custom|DeactivateParticle
  (bind _niagarasystem (Variables|Default|GetNiagaraSystem))
  (Utilities|IsValid _niagarasystem
    (:Is%20Valid
      (Components|Activation|Deactivate _niagarasystem)
      (Development|PrintString "Deactivate"))))

(event EventBeginPlay
  (CallFunction|SpawnPollenFX)
  (CallFunction|ActivateParticle)
  (Collision|SetActorEnableCollision false))

(fn ConstructionScript)