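; Cutscene actor for StarGardener that plays an assigned level sequence when StartCutscene is called.
; It sets the victory jingle audio state, optionally shows the game logo widget, and switches the ice-skating character's ActiveState for the sequence.
; A delay based on the sequence's view range end times the follow-up character state change.
; If the logo was shown, it is then removed and the garden audio state is set.
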(event Custom|StartCutscene
  (bind _sequence (Variables|Default|GetSequence))
  (Class|AkGameplayStatics|SetState "/Game/WwiseAudio/State/State_Zone_Terrain/State_Zone_Terrain-Jingle_Victory.State_Zone_Terrain-Jingle_Victory")
  (bind _outactor (Sequencer|Player|CreateLevelSequencePlayer _sequence))
  (Sequencer|Player|Play (Variables|/Script/LevelSequence.LevelSequenceActor|GetSequencePlayer _outactor) :!class /Script/MovieScene.MovieSceneSequencePlayer)
  (bind _asbp_character_ice_skating (Utilities|Casting|CastToBP_CharacterIceSkating (Game|Player|GetPlayerPawn 0)))
  (Variables|/Game/StarGardener/Object/CharacterController/BP_CharacterIceSkating.BP_CharacterIceSkating_C|SetActiveState _asbp_character_ice_skating "NewEnumerator5")
  (if (Variables|Default|GetIsLogoNeeded)
    (bind _returnvalue (UserInterface|CreateWidget "/Game/StarGardener/UI/Cutscene/LogoGame.LogoGame_C" (Game|GetPlayerController 0)))
    (UserInterface|Viewport|AddtoViewport _returnvalue 0))
  (Utilities|FlowControl|Delay (Class|MovieSceneSequenceExtensions|GetViewRangeEnd _sequence))
  (Variables|/Game/StarGardener/Object/CharacterController/BP_CharacterIceSkating.BP_CharacterIceSkating_C|SetActiveState _asbp_character_ice_skating "NewEnumerator6")
  (Utilities|IsValid _returnvalue
    (:Is%20Valid
      (Widget|RemovefromParent _returnvalue)
      (Class|AkGameplayStatics|SetState "/Game/WwiseAudio/State/State_Zone_Terrain/State_Zone_Terrain-Garden.State_Zone_Terrain-Garden"))))

(event EventBeginPlay)

(event Collision|EventActorBeginOverlap
  (params (OtherActor :type Actor%20Object%20Reference)))

(event EventTick
  (params (DeltaSeconds :type Float%20%28single-precision%29)))

(fn ConstructionScript)