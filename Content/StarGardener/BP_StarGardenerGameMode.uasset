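; Game mode for StarGardener that acts as a registry of position capture objects and finds the one covering a given position.
; The SetPositionCapture event adds a reference to the PositionCapture array.
; GetPositionCapture returns the first entry whose CheckIfActorInBox test accepts the position, with a validity flag for when no capture is found.
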(event Custom|SetPositionCapture
  (params (ObjectReference :type Position%20Capture%20BP%20Object%20Reference))
  (Utilities|Array|Add (Variables|Default|GetPositionCapture) ObjectReference))

(fn ConstructionScript
  (|CallParentFunction))

(fn GetPositionCapture
  (params (Position :type Vector))
  (bind _array_element (Utilities|Array|ForEachLoopwithBreak (Variables|Default|GetPositionCapture) :!label _label)
    (:LoopBody
      (bind _isinbox (Default|CheckifActorinBox _array_element Position))
      (if _isinbox
        (LocalVariables|SetSceneCapture _array_element)
        (goto _label Break)))
    (:Completed
      (Utilities|IsValid (LocalVariables|GetSceneCapture)
        (:Is%20Valid
          (return (LocalVariables|GetSceneCapture) true))
        (:Is%20Not%20Valid
          (return 0 false))))))