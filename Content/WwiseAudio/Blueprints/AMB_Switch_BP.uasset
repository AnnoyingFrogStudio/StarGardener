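; Wwise ambience trigger volume that sets an audio state when the player pawn enters its box.
; With IsJingle set, it first applies the garden-start jingle state, waits, then applies its configured state and clears the flag.
; A DoOnce, reset when the player exits, guards re-triggering.
; Instances flagged MusicBegin also post Play_Music on BeginPlay; the SetSwitch nodes are disconnected.
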(event OnComponentBeginOverlap(Box)
  (params (OverlappedComponent :type Primitive%20Component%20Object%20Reference) (OtherActor :type Actor%20Object%20Reference) (OtherComp :type Primitive%20Component%20Object%20Reference) (OtherBodyIndex :type Integer) (bFromSweep :type Boolean) (SweepResult :type Hit%20Result%20Structure%20%28by%20ref%29))
  ;[0.0317 1 0.3512] AMB State
  (if (== OtherActor (Game|Player|GetPlayerPawn 0))
    (Utilities|FlowControl|DoOnce false
      (:Completed
        (if (Variables|Default|GetIsJingle)
          (Class|AkGameplayStatics|SetState "/Game/WwiseAudio/State/State_Zone_Terrain/State_Zone_Terrain-Jingle_StartGarden.State_Zone_Terrain-Jingle_StartGarden")
          (Utilities|FlowControl|Delay 13.0)
          (Class|AkGameplayStatics|SetState (Variables|Default|GetState%20Value_0))
          (Development|PrintString "GANRDEN" true true "(R=1.000000,G=0.000000,B=0.036360,A=1.000000)")
          (Variables|Default|SetIsJingle false)
          (else
            (Class|AkGameplayStatics|SetState (Variables|Default|GetState%20Value_0))))
        (Variables|Default|SetSwitch_NoEdit (Variables|Default|GetSwitch%20Value))))))

(event OnComponentEndOverlap(Box)
  (params (OverlappedComponent :type Primitive%20Component%20Object%20Reference) (OtherActor :type Actor%20Object%20Reference) (OtherComp :type Primitive%20Component%20Object%20Reference) (OtherBodyIndex :type Integer))
  ;[0.0317 1 0.3512] AMB State
  (if (== OtherActor (Game|Player|GetPlayerPawn 0))
    (Utilities|FlowControl|DoOnce false) ; enters at Reset
  ))

(event EventBeginPlay
  (if (Variables|Default|GetMusic%20Begin)
    (Class|AkGameplayStatics|SetOcclusionRefreshInterval 0.0 self)
    (Class|AkGameplayStatics|PostEvent "/Game/WwiseAudio/Events/MUSIC/Play_Music.Play_Music")))

(fn ConstructionScript)