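; Wwise audio zone actor that starts the Play_Music event on BeginPlay and changes its switch when the player pawn enters its box trigger.
; If IsJingle is set, the first entry switches to the start-garden jingle, waits out a fixed delay, applies the instance-editable SwitchValue, then clears the flag.
; Otherwise it applies SwitchValue immediately, with a DoOnce that resets when the player leaves the box.
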(event OnComponentBeginOverlap(Box)
  (params (OverlappedComponent :type Primitive%20Component%20Object%20Reference) (OtherActor :type Actor%20Object%20Reference) (OtherComp :type Primitive%20Component%20Object%20Reference) (OtherBodyIndex :type Integer) (bFromSweep :type Boolean) (SweepResult :type Hit%20Result%20Structure%20%28by%20ref%29))
  (bind _self self)
  ;[0.0317 1 0.3512] AMB State
  (if (== OtherActor (Game|Player|GetPlayerPawn 0))
    (Utilities|FlowControl|DoOnce false
      (:Completed
        (if (Variables|Default|GetIsJingle)
          (Class|AkGameplayStatics|SetSwitch "/Game/WwiseAudio/Switches/Zone_Terrain/Zone_Terrain-Jingle_StartGarden.Zone_Terrain-Jingle_StartGarden" _self "" "")
          (Utilities|FlowControl|Delay 13.0)
          ;[1 0.439 0.6429] Instance Editable
          (Class|AkGameplayStatics|SetSwitch (Variables|Default|GetSwitch%20Value) _self)
          (Variables|Default|SetIsJingle false)
          (else
            ;;[1 0.439 0.6429] Instance Editable
            (Class|AkGameplayStatics|SetSwitch (Variables|Default|GetSwitch%20Value) _self)))))))

(event OnComponentEndOverlap(Box)
  (params (OverlappedComponent :type Primitive%20Component%20Object%20Reference) (OtherActor :type Actor%20Object%20Reference) (OtherComp :type Primitive%20Component%20Object%20Reference) (OtherBodyIndex :type Integer))
  (bind _self self)
  ;[0.0317 1 0.3512] AMB State
  (if (== OtherActor (Game|Player|GetPlayerPawn 0))
    (Utilities|FlowControl|DoOnce false) ; enters at Reset
  ))

(event EventBeginPlay
  (Class|AkGameplayStatics|PostEvent "/Game/WwiseAudio/Events/MUSIC/Play_Music.Play_Music" self))

(fn ConstructionScript)